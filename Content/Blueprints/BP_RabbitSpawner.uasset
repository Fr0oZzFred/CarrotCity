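; BP_RabbitSpawner spawns Rabbit actors at a randomly chosen one of five origin nodes.
; Tick counts down two independent cooldown timers: one releases a single rabbit, the other a wave of several, re-rolling the node for each.
; Each rabbit spawns at its node's transform and receives that node as its CurrentNode.
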(event EventBeginPlay)

(event Collision|EventActorBeginOverlap
  (params (OtherActor :type Actor%20Object%20Reference)))

(event EventTick
  (params (DeltaSeconds :type Float%20%28single-precision%29))
  (if (< (Variables|Default|GetSpawnTimer) 0.0)
    (Variables|Default|SetSpawnTimer (Variables|Default|GetSpawnCooldown))
    (Variables|Default|SetSpawnIndex (Math|Random|RandomIntegerinRange 0 4))
    (Game|SpawnActorfromClass (Variables|Default|GetRabbit) (Transformation|GetActorTransform (Utilities|Select :Index (Variables|Default|GetSpawnIndex) :Option%200 (Variables|Default|GetOriginNode1) :Option%201 (Variables|Default|GetOriginNode2) :Option%202 (Variables|Default|GetOriginNode3) :Option%203 (Variables|Default|GetOriginNode4) :Option%204 (Variables|Default|GetOriginNode5))) "Undefined" "SelectDefaultAtRuntime" 0 (Utilities|Select :Index (Variables|Default|GetSpawnIndex) :Option%200 (Variables|Default|GetOriginNode1) :Option%201 (Variables|Default|GetOriginNode2) :Option%202 (Variables|Default|GetOriginNode3) :Option%203 (Variables|Default|GetOriginNode4) :Option%204 (Variables|Default|GetOriginNode5)) false 0)
    (else
      (Variables|Default|SetSpawnTimer (- (Variables|Default|GetSpawnTimer) DeltaSeconds))))
  (if (< (Variables|Default|GetWaveSpawnTimer) 0.0)
    (Variables|Default|SetWaveSpawnTimer (Variables|Default|GetWaveSpawnCooldown))
    (for _index (range 0 3)
      (Variables|Default|SetSpawnIndex (Math|Random|RandomIntegerinRange 0 4))
      (Game|SpawnActorfromClass (Variables|Default|GetRabbit) (Transformation|GetActorTransform (Utilities|Select :Index (Variables|Default|GetSpawnIndex) :Option%200 (Variables|Default|GetOriginNode1) :Option%201 (Variables|Default|GetOriginNode2) :Option%202 (Variables|Default|GetOriginNode3) :Option%203 (Variables|Default|GetOriginNode4) :Option%204 (Variables|Default|GetOriginNode5))) "Undefined" "SelectDefaultAtRuntime" 0 (Utilities|Select :Index (Variables|Default|GetSpawnIndex) :Option%200 (Variables|Default|GetOriginNode1) :Option%201 (Variables|Default|GetOriginNode2) :Option%202 (Variables|Default|GetOriginNode3) :Option%203 (Variables|Default|GetOriginNode4) :Option%204 (Variables|Default|GetOriginNode5)) false 0))
    (else
      (Variables|Default|SetWaveSpawnTimer (- (Variables|Default|GetWaveSpawnTimer) DeltaSeconds)))))

(fn ConstructionScript)