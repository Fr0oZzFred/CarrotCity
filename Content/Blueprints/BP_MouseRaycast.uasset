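; Input actor that turns player touches into world interactions with fences and rabbits.
; On touch, it line-traces from the deprojected cursor position and acts on the hit actor according to BP_GameMode's click mode.
; None mode toggles active, unobstructed fences, Fence mode toggles fences under a placement cooldown, and Carrot mode stuns rabbits under a stun cooldown or toggles active fences.
; A debug key increments the game mode's lost count.
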(event EventBeginPlay
  (Input|EnableInput (Game|GetPlayerController 0))
  (Variables|Default|SetGameMode (.AsBP%20Game%20Mode (Utilities|Casting|CastToBP_GameMode (Game|GetGameMode)))))

(event Input|KeyboardEvents|DebugKey<
  (params (Key :type Key%20Structure :default "None") (ActionValue :type Input%20Action%20Value%20Structure))
  (:Pressed
    (Default|IncreasedLost (Variables|Default|GetGameMode))))

(event Input|TouchEvents|Touch1
  (params (Key :type Key%20Structure :default "None"))
  (bind _gamemode (Variables|Default|GetGameMode))
  (bind _gamemode_2 (Variables|Default|GetGameMode))
  (bind _gamemode_3 (Variables|Default|GetGameMode))
  (:Pressed
    (switch Utilities|FlowControl|Switch|SwitchonE_ClickMode (Variables|/Game/Blueprints/BP_GameMode.BP_GameMode_C|GetCurrentClickMode (Variables|Default|GetGameMode))
      (:NewEnumerator0
        (bind _hitactor (CallFunction|DrawRaycast))
        (bind _asbp_fence (Utilities|Casting|CastToBP_Fence _hitactor))
        (if (and (Variables|/Game/Fence/BP_Fence.BP_Fence_C|GetActive _asbp_fence) (not (Variables|/Game/Fence/BP_Fence.BP_Fence_C|GetObstacleActive _asbp_fence)))
          (Default|Place/Remove _asbp_fence)
          (Default|CallOnClickModeChanged (Variables|Default|GetGameMode) "NewEnumerator0") ; Used to reset anim on ui
        ))
      (:NewEnumerator2
        (if (>= (Variables|/Game/Blueprints/BP_GameMode.BP_GameMode_C|GetPlacementTimer _gamemode_3) (Variables|/Game/Blueprints/BP_GameMode.BP_GameMode_C|GetPlacementCooldown _gamemode_3))
          (bind _hitactor_2 (CallFunction|DrawRaycast))
          (bind _asbp_fence_2 (Utilities|Casting|CastToBP_Fence _hitactor_2))
          (if (not (Variables|/Game/Fence/BP_Fence.BP_Fence_C|GetObstacleActive _asbp_fence_2))
            (Default|Place/Remove _asbp_fence_2)
            (Default|SetClickMode (Variables|Default|GetGameMode) "NewEnumerator0"))))
      (:NewEnumerator1
        (if (>= (Variables|/Game/Blueprints/BP_GameMode.BP_GameMode_C|GetStunTimer _gamemode_2) (Variables|/Game/Blueprints/BP_GameMode.BP_GameMode_C|GetStunCooldown _gamemode_2))
          (bind _hitactor_3 (CallFunction|DrawRaycast))
          (bind _asbp_rabbit (Utilities|Casting|CastToBP_Rabbit _hitactor_3)
            (:then
              (Default|Stun _asbp_rabbit)
              (Variables|/Game/Blueprints/BP_GameMode.BP_GameMode_C|SetStunTimer _gamemode 0.0)
              (Default|SetClickMode _gamemode "NewEnumerator0"))
            (:CastFailed
              (bind _asbp_fence_3 (Utilities|Casting|CastToBP_Fence _hitactor_3))
              (if (Variables|/Game/Fence/BP_Fence.BP_Fence_C|GetActive _asbp_fence_3)
                (Default|Place/Remove _asbp_fence_3)))))))))

(fn ConstructionScript)

(fn DrawRaycast
  (bind _returnvalue (Game|GetPlayerController 0))
  (bind (_worldlocation _worlddirection) (Game|Player|ConvertMouseLocationToWorldSpace _returnvalue))
  (bind _outhit (Collision|LineTraceByChannel _worldlocation (+ _worldlocation (* _worlddirection 7e+03)) "TraceTypeQuery1" false 0 "None"))
  (return (.HitActor (Collision|BreakHitResult _outhit))))