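; BP_SpawnManager spawns rabbits at placed spawn points, each with a pop sound and a scale animation on the matching house.
; BeginPlay spawns a first bunny, shows the tutorial widget and pauses, then starts a self-calling delay loop that shortens each wait.
; Random picks avoid repeating the last point and switch to the least-used one when counts drift apart.
; Fat bunnies appear after enough saves, randomly or forced after a dry streak.
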(event Custom|SpawnBunnyWithDelay
  (params (DelayDuration :type Float%20%28double-precision%29) (Loop :type Boolean))
  (Utilities|FlowControl|Delay DelayDuration)
  (CallFunction|SpawnBunnyRnd)
  (if Loop
    (CallFunction|SpawnBunnywithDelay (- DelayDuration 0.1) Loop)))

(event Custom|PlayHouseSpawnAnim
  (Audio|PlaySound2D (.OutItem (Utilities|Array|Random (Utilities|Array|MakeArray "/Game/Sounds/3pops/pop1.pop1" "/Game/Sounds/pop.pop" "/Game/Sounds/3pops/pop3.pop3"))) 1.0 1.0 0.0 0 0)
  (bind _scale (Timeline|Timeline PlayFromStart)
    (:Update
      (Transformation|SetActorScale3D (Utilities|Array|Get(acopy) (Variables|Default|GetHouses) (Variables|Default|GetLastSpawnedIdx)) _scale))))

(event EventBeginPlay
  ;[1 1 1] Init
  (for _array_element (Variables|Default|GetSpawnPoints)
    (Utilities|Array|Add (Variables|Default|GetSpawnLocations) (Transformation|GetActorLocation _array_element))
    (Utilities|Array|Add (Variables|Default|GetSpawnCount) 0))
  (Utilities|FlowControl|Delay 2.0)
  (CallFunction|SpawnBunny 2 false)
  (Utilities|FlowControl|Delay 1.0)
  (bind _returnvalue (UserInterface|CreateWidget "/Game/Widgets/UMG_BaseTuto.UMG_BaseTuto_C"))
  (UserInterface|Viewport|AddtoViewport _returnvalue 0)
  (Game|SetGamePaused true)
  (Utilities|FlowControl|Delay 4.0)
  (CallFunction|SpawnBunnywithDelay (Variables|Default|GetDelayTimer) true))

(event EventTick
  (params (DeltaSeconds :type Float%20%28single-precision%29)))

(fn ConstructionScript)

(fn SpawnBunny
  (params (SpawnIndex :type Integer) (FatBunny :type Boolean))
  (Variables|Default|SetLastSpawnedWasFat FatBunny)
  (bind _output_get (Variables|Default|SetLastSpawnedIdx SpawnIndex))
  (Game|SpawnActorfromClass "/Game/Rabbits/BP_Rabbit.BP_Rabbit_C" (Math|Transform|MakeTransform (Transformation|GetActorLocation (Utilities|Array|Get(acopy) (Variables|Default|GetSpawnPoints) _output_get)) "0, 0, 0" "1.000000,1.000000,1.000000") "Undefined" 0 (Utilities|Array|Get(acopy) (Variables|Default|GetSpawnPoints) _output_get) FatBunny 0)
  (CallFunction|PlayHouseSpawnAnim))

(fn SpawnBunnyRnd
  ;[1 1 1] Get Min and Max Index
  (for (_array_element _array_index) (Variables|Default|GetSpawnCount)
    (Utilities|FlowControl|Sequence
      (:then_0
        (if (< _array_element (Utilities|Array|Get(acopy) (Variables|Default|GetSpawnCount) (LocalVariables|GetMinIdx)))
          (LocalVariables|SetMinIdx _array_index)))
      (:then_1
        (if (> _array_element (Utilities|Array|Get(acopy) (Variables|Default|GetSpawnCount) (LocalVariables|GetMaxIdx)))
          (LocalVariables|SetMaxIdx _array_index)))))
  ;[1 1 1] Check the difference of spawn count
  (if (<= (- (Utilities|Array|Get(acopy) (Variables|Default|GetSpawnCount) (LocalVariables|GetMaxIdx)) (Utilities|Array|Get(acopy) (Variables|Default|GetSpawnCount) (LocalVariables|GetMinIdx))) 3)
    ;[1 1 1] Rnd Idx
    (bind _output_get (LocalVariables|SetSpawnIdx (Math|Random|RandomInteger (Utilities|Array|Length (Variables|Default|GetSpawnPoints)))))
    (while (== _output_get (Variables|Default|GetLastSpawnedIdx))
      (LocalVariables|SetSpawnIdx (Math|Random|RandomInteger (Utilities|Array|Length (Variables|Default|GetSpawnPoints)))))
    (else
      (LocalVariables|SetSpawnIdx (LocalVariables|GetMinIdx))))
  (LocalVariables|SetFatBunny (select (< (Variables|/Game/Blueprints/BP_GameMode.BP_GameMode_C|GetSavedBunnies (.AsBP%20Game%20Mode (Utilities|Casting|CastToBP_GameMode (Game|GetGameMode)))) 6) false (select (>= (Variables|Default|GetCountSinceLastFat) 6) true (> (Math|Random|RandomInteger 6) 4))))
  (CallFunction|SpawnBunny (LocalVariables|GetSpawnIdx) (LocalVariables|GetFatBunny))
  (Math|Integer|IncrementInt (Utilities|Array|Get(acopy) (Variables|Default|GetSpawnCount) (LocalVariables|GetSpawnIdx))
    (:%20%20
      (if (not (LocalVariables|GetFatBunny))
        (Math|Integer|IncrementInt (Variables|Default|GetCountSinceLastFat))
        (else
          (Variables|Default|SetCountSinceLastFat 0))))))