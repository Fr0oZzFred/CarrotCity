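; BP_PathNode is a route waypoint that pairs with a Neighbour node and manages the barrier between them.
; On BeginPlay it waits for a valid Neighbour, then spawns one shared BP_Fence at their midpoint and links both nodes.
; Obstacle nodes use randomized Tick timers to trigger the barrier's tree-fall or removal animations, depending on IsActive.
; Routing functions return an eligible Neighbour other than the departure node, falling back to Forward.
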(event Custom|SpawnObstacle
  (bind _barrier (Variables|Default|GetBarrier))
  (if (not (Audio|Components|Audio|IsPlaying (Variables|/Game/Fence/BP_Fence.BP_Fence_C|GetTreeStartFalling _barrier)))
    (Default|StartFallingAnim _barrier)
    (Utilities|FlowControl|Delay 4.0)
    (bind _reachend (Default|ChangeObstacle (Variables|Default|GetBarrier) true :!label _label))
    (if _reachend
      (Variables|Default|SetObstacleTimer (Math|Random|RandomFloatinRange 1e+01 3e+01))
      (else
        (Utilities|FlowControl|DelayUntilNextTick)
        (goto _label)))))

(event Custom|RemoveObstacle
  (if (not (Audio|Components|Audio|IsPlaying (Variables|/Game/Fence/BP_Fence.BP_Fence_C|GetRemoveTreeAnim (Variables|Default|GetBarrier))))
    (Default|StartTreeRemoveAnim (Variables|Default|GetBarrier))
    (Utilities|FlowControl|Delay 4.0)
    (Default|ChangeObstacle (Variables|Default|GetBarrier) false)
    (Variables|Default|SetObstacleTimer (Math|Random|RandomFloatinRange 3e+01 1e+02))))

(event EventBeginPlay
  (bind _returnvalue (Transformation|GetActorLocation))
  (Utilities|IsValid (Variables|Default|GetNeighbour) :!label _label
    (:Is%20Valid
      (if (not (Utilities|IsValid (Variables|Default|GetBarrier)))
        (bind _returnvalue_2 (Game|SpawnActorfromClass "/Game/Fence/BP_Fence.BP_Fence_C" (Math|Transform|MakeTransform (+ _returnvalue (* (Math|Vector|GetForwardVector (Math|Rotator|FindLookatRotation _returnvalue (Transformation|GetActorLocation (Variables|Default|GetNeighbour)))) (/ (Math|Vector|Distance(Vector) _returnvalue (Transformation|GetActorLocation (Variables|Default|GetNeighbour))) 2.0))) (Math|Rotator|FindLookatRotation _returnvalue (Transformation|GetActorLocation (Variables|Default|GetNeighbour))) "1.000000,1.000000,1.000000") "Undefined" "OverrideRootScale" 0 (Variables|Default|GetNeighbour) 0))
        (bind _output_get (Variables|Default|SetBarrier _returnvalue_2))
        (Variables|BP_PathNode_C|SetBarrier (Variables|Default|GetNeighbour) _output_get)
        (Variables|BP_PathNode_C|SetNeighbour (Variables|Default|GetNeighbour) self)
        (if (Variables|Default|GetIsObstacle)
          (bind _output_get_2 (Variables|Default|SetObstacleCooldown (Math|Random|RandomFloatinRange 45.0 75.0)))
          (Variables|Default|SetObstacleTimer _output_get_2))))
    (:Is%20Not%20Valid
      (Utilities|FlowControl|DelayUntilNextTick)
      (goto _label))))

(event Collision|EventActorBeginOverlap
  (params (OtherActor :type Actor%20Object%20Reference)))

(event EventTick
  (params (DeltaSeconds :type Float%20%28single-precision%29))
  (if (Variables|Default|GetIsObstacle)
    (if (> (Variables|Default|GetObstacleTimer) 0.0)
      (Variables|Default|SetObstacleTimer (- (Variables|Default|GetObstacleTimer) DeltaSeconds))
      (elif (Variables|Default|GetIsActive)
        (CallFunction|SpawnObstacle)
        (else
          (CallFunction|RemoveObstacle))))))

(fn ConstructionScript)

(fn GetOpenNeighbour
  (params (DepartureNode :type BP%20Path%20Node%20Object%20Reference))
  (bind _forward (Variables|Default|GetForward))
  (bind _neighbour (Variables|Default|GetNeighbour))
  (Utilities|IsValid _neighbour
    (:Is%20Valid
      (if (Math|Boolean|ANDBoolean (Variables|BP_PathNode_C|GetIsOpen _neighbour) (Variables|BP_PathNode_C|GetIsActive _neighbour) (not (== _neighbour DepartureNode)))
        (return _neighbour)
        (else
          _)))
    (:Is%20Not%20Valid
      _))
  (Utilities|IsValid _forward
    (:Is%20Valid
      (return _forward))
    (:Is%20Not%20Valid
      (return 0))))

(fn GetActiveNeighbour
  (params (DepartureNode :type BP%20Path%20Node%20Object%20Reference))
  (bind _forward (Variables|Default|GetForward))
  (bind _neighbour (Variables|Default|GetNeighbour))
  (Utilities|IsValid _neighbour
    (:Is%20Valid
      (if (and (Variables|BP_PathNode_C|GetIsActive _neighbour) (not (== _neighbour DepartureNode)))
        (return _neighbour)
        (else
          _)))
    (:Is%20Not%20Valid
      _))
  (Utilities|IsValid _forward
    (:Is%20Valid
      (return _forward))
    (:Is%20Not%20Valid
      (return 0))))