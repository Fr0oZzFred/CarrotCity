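; BP_GameMode is a game mode that manages a limited barrier stock and cooldown timers for barrier placement and stun.
; BeginPlay shows the mouse cursor and fills the stock to its maximum, while Tick advances both timers toward their cooldowns.
; PlaceBarrier requires a finished placement cooldown, then spends or refunds one barrier, resets that timer and returns success.
; The stun timer only counts up here; nothing in this Blueprint resets or reads it for gameplay.
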(event EventBeginPlay
  (Variables|/Script/Engine.PlayerController|SetbShowMouseCursor (Game|GetPlayerController 0) true)
  (Variables|Default|SetStockBarrier (Variables|Default|GetMaxBarrier)))

(event EventTick
  (params (DeltaSeconds :type Float%20%28single-precision%29))
  (bind _placementcooldown (Variables|Default|GetPlacementCooldown))
  (bind _stuncooldown (Variables|Default|GetStunCooldown))
  (if (!= (Variables|Default|GetPlacementTimer) _placementcooldown)
    (if (< (Variables|Default|GetPlacementTimer) _placementcooldown)
      (Variables|Default|SetPlacementTimer (+ (Variables|Default|GetPlacementTimer) DeltaSeconds))
      (else
        (Variables|Default|SetPlacementTimer (Variables|Default|GetPlacementCooldown)))))
  (if (!= (Variables|Default|GetStunTimer) _stuncooldown)
    (if (< (Variables|Default|GetStunTimer) _stuncooldown)
      (Variables|Default|SetStunTimer (+ (Variables|Default|GetStunTimer) DeltaSeconds))
      (else
        (Variables|Default|SetStunTimer (Variables|Default|GetStunCooldown))))))

(fn ConstructionScript)

(fn PlaceBarrier
  (params (Placing :type Boolean))
  (bind _stockbarrier (Variables|Default|GetStockBarrier))
  (if (>= (Variables|Default|GetPlacementTimer) (Variables|Default|GetPlacementCooldown))
    (if Placing
      (if (> _stockbarrier 0)
        (Math|Integer|DecrementInt _stockbarrier
          (:%20%20
            _))
        (else
          (return false)))
      (else
        (Math|Integer|IncrementInt _stockbarrier
          (:%20%20
            _))))
    (Variables|Default|SetPlacementTimer 0.0)
    (return true)
    (else
      (return false))))