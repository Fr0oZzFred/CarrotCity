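; BP_GI, apparently the Game Instance, handles main theme music, level loading and the current game state.
; The looping theme is created once as a 2D sound that persists across level transitions.
; OpenLevel opens a level, adds a loading widget a tick later and removes it after a random delay of a few seconds, independent of actual load progress.
; SetGameState calls OnGameStateChanged only when the state changes.
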(event Custom|PlayMainTheme
  (Utilities|IsValid (Variables|Default|GetMainTheme)
    (:Is%20Not%20Valid
      (bind _returnvalue (Audio|CreateSound2D "/Game/Sounds/CUE_Bunny_Dust_Looped.CUE_Bunny_Dust_Looped" 1.0 1.0 0.0 0 true))
      (bind _output_get (Variables|Default|SetMainTheme _returnvalue))
      (Audio|Components|Audio|Play _output_get 0.0))))

(event Custom|OpenLevel
  (params (Level :type World%20Soft%20Object%20Reference))
  (Game|OpenLevel(byObjectReference) Level)
  (Utilities|FlowControl|DelayUntilNextTick)
  (bind _returnvalue (UserInterface|CreateWidget "/Game/Widgets/UMG_Loading.UMG_Loading_C"))
  (bind _output_get (Variables|Default|SetLoading_HUD _returnvalue))
  (UserInterface|Viewport|AddtoViewport _output_get 0)
  (Utilities|FlowControl|Delay (Math|Random|RandomFloatinRange 3.0 4.0))
  (Widget|RemovefromParent (Variables|Default|GetLoading_HUD))
  (Variables|Default|SetLoading_HUD 0))

(fn SetGameState
  (params (NewGameState :type E_GameState%20Enum :default "NewEnumerator0"))
  (if (Utilities|Enum|NotEqual(Enum) NewGameState (Variables|Default|GetCurrentGameState))
    (bind _output_get (Variables|Default|SetCurrentGameState NewGameState))
    (Default|CallOnGameStateChanged _output_get)))