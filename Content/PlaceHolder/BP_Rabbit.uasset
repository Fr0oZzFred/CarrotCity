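; BP_Rabbit is a rabbit actor that walks a node network and adds to the game mode's saved or lost bunny count when its path ends.
; Tick moves it toward the current node, then asks that node for an open neighbour, notifying any barrier shared by both nodes as it crosses.
; Stun zeroes its speed until a timer expires.
; FatBunny only tints it red instead of white.
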(event EventBeginPlay
  (Rendering|Material|SetVectorParameterValueonMaterials (Variables|Default|GetBody) "Color" (select (Variables|Default|GetFatBunny) "1.000000,0.000000,0.000000" "1.000000,1.000000,1.000000"))
  (Variables|Default|SetUseSpeed (Variables|Default|GetSpeed)))

(event EventTick
  (params (DeltaSeconds :type Float%20%28single-precision%29))
  (if (!= (Variables|Default|GetStunTimer) 0.0)
    (if (> (Variables|Default|GetStunTimer) 0.0)
      (Variables|Default|SetStunTimer (- (Variables|Default|GetStunTimer) DeltaSeconds))
      (else
        (Variables|Default|SetUseSpeed (Variables|Default|GetSpeed))
        (Variables|Default|SetStunTimer 0.0))))
  (Utilities|IsValid (Variables|Default|GetCurrentNode)
    (:Is%20Valid
      (Transformation|SetActorRotation (Math|Rotator|FindLookatRotation (Transformation|GetActorLocation) (Transformation|GetActorLocation (Variables|Default|GetCurrentNode))))
      (Transformation|SetActorLocation (+ (Transformation|GetActorLocation) (* (Transformation|GetActorForwardVector) (Variables|Default|GetUseSpeed))) true false)
      (if (< (Math|Vector|Distance(Vector) (Transformation|GetActorLocation) (Transformation|GetActorLocation (Variables|Default|GetCurrentNode))) 1e+01)
        (Utilities|IsValid (Variables|Default|GetCurrentBarrier)
          (:Is%20Valid
            (Default|ChangeRabbit (Variables|Default|GetCurrentBarrier) false)
            (Variables|Default|SetCurrentBarrier 0))
          (:Is%20Not%20Valid
            _))
        (bind _newtargetnode (Default|GetOpenNeighbour (Variables|Default|GetCurrentNode) (Variables|Default|GetOldNode)))
        (bind _output_get (Variables|Default|SetOldNode (Variables|Default|GetCurrentNode)))
        (if (!= _output_get _newtargetnode)
          (bind _output_get_2 (Variables|Default|SetCurrentNode _newtargetnode))
          (Utilities|IsValid _output_get_2
            (:Is%20Valid
              (Utilities|IsValid (Variables|/Game/PlaceHolder/BP_PathNode.BP_PathNode_C|GetBarrier _output_get_2)
                (:Is%20Valid
                  (if (== (Variables|/Game/PlaceHolder/BP_PathNode.BP_PathNode_C|GetBarrier _output_get_2) (Variables|/Game/PlaceHolder/BP_PathNode.BP_PathNode_C|GetBarrier (Variables|Default|GetOldNode)))
                    (bind _output_get_3 (Variables|Default|SetCurrentBarrier (Variables|/Game/PlaceHolder/BP_PathNode.BP_PathNode_C|GetBarrier _output_get_2)))
                    (Default|ChangeRabbit _output_get_3 true)))))
            (:Is%20Not%20Valid
              (CallFunction|EndPath))))))
    (:Is%20Not%20Valid
      (CallFunction|EndPath))))

(fn ConstructionScript)

(fn Stun
  (Variables|Default|SetStunTimer (Variables|Default|GetStunCooldown))
  (Variables|Default|SetUseSpeed 0.0)
  (Development|PrintString "rabbit stun"))

(fn EndPath
  (bind _asbp_game_mode (Utilities|Casting|CastToBP_GameMode (Game|GetGameMode)))
  (if (Variables|/Game/PlaceHolder/BP_PathNode.BP_PathNode_C|GetIsWin (Variables|Default|GetOldNode))
    (Math|Integer|IncrementInt (Variables|/Game/Blueprints/BP_GameMode.BP_GameMode_C|GetSavedBunnies _asbp_game_mode)
      (:%20%20
        _)))
  (if (Variables|/Game/PlaceHolder/BP_PathNode.BP_PathNode_C|GetIsLose (Variables|Default|GetOldNode))
    (Math|Integer|IncrementInt (Variables|/Game/Blueprints/BP_GameMode.BP_GameMode_C|GetLostBunnies _asbp_game_mode)
      (:%20%20
        _)))
  (Actor|DestroyActor))