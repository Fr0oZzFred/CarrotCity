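; BP_Barrier is a placeholder barrier actor that blocks or opens a linked node.
; Its cube mesh is hidden on BeginPlay.
; Two debug keys toggle it: one shows the cube and sets LinkedNode.IsOpen to false, the other hides it and reopens the node, each printing a status message.
; Only cube visibility changes; collision is untouched.
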(event EventBeginPlay
  (Rendering|SetVisibility (Variables|Default|GetCube) false false))

(event Collision|EventActorBeginOverlap
  (params (OtherActor :type Actor%20Object%20Reference)))

(event EventTick
  (params (DeltaSeconds :type Float%20%28single-precision%29)))

(event Input|KeyboardEvents|DebugKeyA
  (params (Key :type Key%20Structure :default "None") (ActionValue :type Input%20Action%20Value%20Structure))
  (:Pressed
    (Development|PrintString "active")
    (Rendering|SetVisibility (Variables|Default|GetCube) true false)
    (Variables|/Game/PlaceHolder/BP_PathNode.BP_PathNode_C|SetIsOpen (Variables|Default|GetLinkedNode) false)))

(event Input|KeyboardEvents|DebugKeyE
  (params (Key :type Key%20Structure :default "None") (ActionValue :type Input%20Action%20Value%20Structure))
  (:Pressed
    (Development|PrintString "deactive")
    (Rendering|SetVisibility (Variables|Default|GetCube) false false)
    (Variables|/Game/PlaceHolder/BP_PathNode.BP_PathNode_C|SetIsOpen (Variables|Default|GetLinkedNode) true)))

(fn ConstructionScript)