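; BP_RabbitSpawner is a placeholder actor that repeatedly spawns Rabbit actors at its own transform.
; Tick counts down two independent timers, SpawnTimer and WaveSpawnTimer, each reset to its own cooldown when it drops below zero.
; Both timers spawn a single Rabbit on expiry, so the wave timer differs only in the cooldown variable it uses.
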(event EventBeginPlay)

(event Collision|EventActorBeginOverlap
  (params (OtherActor :type Actor%20Object%20Reference)))

(event EventTick
  (params (DeltaSeconds :type Float%20%28single-precision%29))
  (if (< (Variables|Default|GetSpawnTimer) 0.0)
    (Variables|Default|SetSpawnTimer (Variables|Default|GetSpawnCooldown))
    (Game|SpawnActorfromClass (Variables|Default|GetRabbit) (Transformation|GetActorTransform) "Undefined" 0 0 0)
    (else
      (Variables|Default|SetSpawnTimer (- (Variables|Default|GetSpawnTimer) DeltaSeconds))))
  (if (< (Variables|Default|GetWaveSpawnTimer) 0.0)
    (Variables|Default|SetWaveSpawnTimer (Variables|Default|GetWaveSpawnCooldown))
    (Game|SpawnActorfromClass (Variables|Default|GetRabbit) (Transformation|GetActorTransform) "Undefined" 0 0 0)
    (else
      (Variables|Default|SetWaveSpawnTimer (- (Variables|Default|GetWaveSpawnTimer) DeltaSeconds)))))

(fn ConstructionScript)