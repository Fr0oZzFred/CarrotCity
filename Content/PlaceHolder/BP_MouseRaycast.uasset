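; BP_MouseRaycast is a placeholder actor that turns mouse clicks into world interactions with fences and rabbits.
; It enables its own input on BeginPlay, then deprojects the cursor and runs a fixed-length Visibility line trace on each click.
; Left click calls PlaceRemove on a hit BP_Fence, and right click calls Stun on a hit BP_Rabbit.
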(event EventBeginPlay
  (Input|EnableInput (Game|GetPlayerController 0)))

(event EventTick
  (params (DeltaSeconds :type Float%20%28single-precision%29)))

(event Input|MouseEvents|LeftMouseButton
  (params (Key :type Key%20Structure))
  (bind _returnvalue (Game|GetPlayerController 0))
  (bind (_worldlocation _worlddirection) (Game|Player|ConvertMouseLocationToWorldSpace _returnvalue))
  (:Pressed
    (bind _outhit (Collision|LineTraceByChannel _worldlocation (+ _worldlocation (* _worlddirection 7e+03)) "TraceTypeQuery1" false 0 "None"))
    (bind _asbp_fence (Utilities|Casting|CastToBP_Fence (.HitActor (Collision|BreakHitResult _outhit))))
    (Default|Place/Remove _asbp_fence)))

(event Input|MouseEvents|RightMouseButton
  (params (Key :type Key%20Structure))
  (bind _returnvalue (Game|GetPlayerController 0))
  (bind (_worldlocation _worlddirection) (Game|Player|ConvertMouseLocationToWorldSpace _returnvalue))
  (:Pressed
    (bind _outhit (Collision|LineTraceByChannel _worldlocation (+ _worldlocation (* _worlddirection 7e+03)) "TraceTypeQuery1" false 0 "None"))
    (bind _asbp_rabbit (Utilities|Casting|CastToBP_Rabbit (.HitActor (Collision|BreakHitResult _outhit))))
    (Default|Stun _asbp_rabbit)))

(fn ConstructionScript)