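; Rabbit actor that walks a node path each Tick, toggling barriers it crosses and reporting saved or lost to BP_GameMode at win or lose nodes.
; Stun halts it to eat a carrot for a cooldown, with a focus VFX following the click mode.
; The FatBunny variant picks active rather than open neighbours and destroys active fences.
; It absorbs stuns until HP runs out, then behaves like a normal rabbit.
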(event Custom|PlayAnimAngry
  (if (Variables|Default|GetFatBunny)
    (bind _angry (Timeline|AngryAnim PlayFromStart)
      (:Update
        (Rendering|Material|SetScalarParameterValueonMaterials (Variables|Default|GetSkeletalMesh) "Angry" _angry)))))

(event Custom|OnClickModeChanged
  (params (NewClickMode :type E_ClickMode%20Enum :default "NewEnumerator0"))
  ;[1 1 1] Init Carrot Focusable
  (Rendering|SetVisibility (Variables|Default|GetVFX_CarrotFocusable) (Utilities|Enum|Equal(Enum) NewClickMode "NewEnumerator1") false))

(event EventBeginPlay
  (bind _skeletalmesh (Variables|Default|GetSkeletalMesh))
  (bind _carrot (Variables|Default|GetCarrot))
  ;[1 1 1] Init Skeletal Mesh
  (Components|SkeletalMesh|SetSkeletalMeshAsset _skeletalmesh (select (Variables|Default|GetFatBunny) "/Game/Rabbits/FatRabbit/FatRabbit.FatRabbit" "/Game/Rabbits/Rabbit/Rabbit.Rabbit"))
  (Class|SkeletalMeshComponent|SetAnimClass _skeletalmesh (select (Variables|Default|GetFatBunny) "/Game/Rabbits/FatRabbit/BA_FatRabbit.BA_FatRabbit_C" "/Game/Rabbits/Rabbit/BA_Rabbit.BA_Rabbit_C"))
  (Variables|Default|SetUseSpeed (Variables|Default|GetSpeed))
  ;[1 1 1] Init Eating Carrot
  (Effects|Components|ParticleSystem|SetFloatParameter (Variables|Default|GetVFX_EatingCarrot) "Duration" (Variables|Default|GetStunCooldown))
  (Transformation|SetRelativeTransform _carrot (Transformation|GetSocketTransform (Variables|Default|GetSkeletalMesh) "CarrotSocket" "RTS_Actor") false false)
  (Development|SetHiddeninGame _carrot true false)
  ;[1 1 1] Init Carrot Focusable
  (bind _output_get (Variables|Default|SetGameMode (.AsBP%20Game%20Mode (Utilities|Casting|CastToBP_GameMode (Game|GetGameMode)))))
  (Rendering|SetVisibility (Variables|Default|GetVFX_CarrotFocusable) (Utilities|Enum|Equal(Enum) (Variables|/Game/Blueprints/BP_GameMode.BP_GameMode_C|GetCurrentClickMode _output_get) "NewEnumerator1") false)
  (EventDispatchers|BindEventtoOnClickModeChanged (Variables|Default|GetGameMode) (delegate Custom|OnClickModeChanged))
  ;[1 1 1] Init angry rabbit vfx
  (if (Variables|Default|GetFatBunny)
    (bind _returnvalue (Niagara|SpawnSystemAttached "/Game/Rabbits/FatRabbit/VFX_FatRabbitAngry.VFX_FatRabbitAngry" (Variables|Default|GetSkeletalMesh) "HeadSocket" "0, 0, 0" "0, 0, 0" "SnapToTargetIncludingScale" false))
    (Variables|Default|SetVFX_AngryRabbit _returnvalue)))

(event Collision|EventActorBeginOverlap
  (params (OtherActor :type Actor%20Object%20Reference))
  (bind _asbp_fence (Utilities|Casting|CastToBP_Fence OtherActor))
  (if (and (Variables|/Game/Fence/BP_Fence.BP_Fence_C|GetActive _asbp_fence) (Variables|Default|GetFatBunny))
    (Default|Destruct _asbp_fence)))

(event EventTick
  (params (DeltaSeconds :type Float%20%28single-precision%29))
  (if (!= (Variables|Default|GetStunTimer) 0.0)
    (if (> (Variables|Default|GetStunTimer) 0.0)
      (Variables|Default|SetStunTimer (- (Variables|Default|GetStunTimer) DeltaSeconds))
      (else
        (Variables|Default|SetUseSpeed (Variables|Default|GetSpeed))
        (Variables|Default|SetStunTimer 0.0)
        (Variables|Default|SetEating false)
        (Development|SetHiddeninGame (Variables|Default|GetCarrot) true false))))
  (Utilities|IsValid (Variables|Default|GetCurrentNode)
    (:Is%20Valid
      (Transformation|SetActorRotation (Math|Rotator|FindLookatRotation (Transformation|GetActorLocation) (Transformation|GetActorLocation (Variables|Default|GetCurrentNode))))
      (Transformation|SetActorLocation (+ (Transformation|GetActorLocation) (* (Transformation|GetActorForwardVector) (Variables|Default|GetUseSpeed) DeltaSeconds)) true false)
      (if (< (Math|Vector|Distance(Vector) (Transformation|GetActorLocation) (Transformation|GetActorLocation (Variables|Default|GetCurrentNode))) 25.0)
        (Utilities|IsValid (Variables|Default|GetCurrentBarrier)
          (:Is%20Valid
            (Default|ChangeRabbit (Variables|Default|GetCurrentBarrier) false)
            (Variables|Default|SetCurrentBarrier 0))
          (:Is%20Not%20Valid
            _))
        (if (not (Variables|Default|GetFatBunny))
          (bind _newtargetnode (Default|GetOpenNeighbour (Variables|Default|GetCurrentNode) (Variables|Default|GetOldNode)))
          (bind _output_get (Variables|Default|SetOldNode (Variables|Default|GetCurrentNode)))
          (if (!= _output_get _newtargetnode)
            (bind _output_get_2 (Variables|Default|SetCurrentNode _newtargetnode))
            (Utilities|IsValid _output_get_2
              (:Is%20Valid
                (Utilities|IsValid (Variables|/Game/Blueprints/BP_PathNode.BP_PathNode_C|GetBarrier _output_get_2)
                  (:Is%20Valid
                    (if (== (Variables|/Game/Blueprints/BP_PathNode.BP_PathNode_C|GetBarrier _output_get_2) (Variables|/Game/Blueprints/BP_PathNode.BP_PathNode_C|GetBarrier (Variables|Default|GetOldNode)))
                      (bind _output_get_3 (Variables|Default|SetCurrentBarrier (Variables|/Game/Blueprints/BP_PathNode.BP_PathNode_C|GetBarrier _output_get_2)))
                      (Default|ChangeRabbit _output_get_3 true)))))
              (:Is%20Not%20Valid
                (CallFunction|EndPath))))
          (else
            (bind _newtargetnode_2 (Default|GetActiveNeighbour (Variables|Default|GetCurrentNode) (Variables|Default|GetOldNode)))
            (bind _output_get_4 (Variables|Default|SetOldNode (Variables|Default|GetCurrentNode)))
            (if (!= _output_get_4 _newtargetnode_2)
              (bind _output_get_5 (Variables|Default|SetCurrentNode _newtargetnode_2))
              (Utilities|IsValid _output_get_5
                (:Is%20Valid
                  (Utilities|IsValid (Variables|/Game/Blueprints/BP_PathNode.BP_PathNode_C|GetBarrier _output_get_5)
                    (:Is%20Valid
                      (if (== (Variables|/Game/Blueprints/BP_PathNode.BP_PathNode_C|GetBarrier _output_get_5) (Variables|/Game/Blueprints/BP_PathNode.BP_PathNode_C|GetBarrier (Variables|Default|GetOldNode)))
                        (bind _output_get_6 (Variables|Default|SetCurrentBarrier (Variables|/Game/Blueprints/BP_PathNode.BP_PathNode_C|GetBarrier _output_get_5)))
                        (Default|ChangeRabbit _output_get_6 true)))))
                (:Is%20Not%20Valid
                  (CallFunction|EndPath))))))))
    (:Is%20Not%20Valid
      (CallFunction|EndPath))))

(fn ConstructionScript)

(fn Stun
  (bind _hp (Variables|Default|GetHP))
  (bind _vfx_angryrabbit (Variables|Default|GetVFX_AngryRabbit))
  (if (Variables|Default|GetFatBunny)
    (Math|Integer|DecrementInt _hp
      (:%20%20
        (if (< _hp 0)
          (Variables|Default|SetFatBunny false)
          (Variables|Default|SetStunTimer (Variables|Default|GetStunCooldown))
          (Variables|Default|SetUseSpeed 0.0)
          (Utilities|IsValid _vfx_angryrabbit
            (:Is%20Valid
              (Components|DestroyComponent _vfx_angryrabbit))
            (:Is%20Not%20Valid
              _))
          (Components|Activation|Activate (Variables|Default|GetVFX_EatingCarrot) true :!label _label)
          (Variables|Default|SetEating true)
          (Development|SetHiddeninGame (Variables|Default|GetCarrot) false false)
          (Audio|PlaySound2D "/Game/Sounds/RabbitEating.RabbitEating" 2.0 1.0 8.0 0 0))))
    (else
      (Variables|Default|SetStunTimer (Variables|Default|GetStunCooldown))
      (Variables|Default|SetUseSpeed 0.0)
      (goto _label))))

(fn EndPath
  (bind _oldnode (Variables|Default|GetOldNode))
  (bind _asbp_game_mode (Utilities|Casting|CastToBP_GameMode (Game|GetGameMode)))
  (if (Variables|/Game/Blueprints/BP_PathNode.BP_PathNode_C|GetIsWin _oldnode)
    (Default|IncreaseSaved _asbp_game_mode)
    (Niagara|SpawnSystematLocation "/Game/Rabbits/VFX_Win.VFX_Win" (Transformation|GetActorLocation _oldnode))
    (Actor|DestroyActor)
    (elif (Variables|/Game/Blueprints/BP_PathNode.BP_PathNode_C|GetIsLose (Variables|Default|GetOldNode))
      (Default|IncreasedLost _asbp_game_mode)
      (Actor|DestroyActor)
      (else
        (Actor|DestroyActor)))))