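; Fence slot on a node link that toggles a barrier from the GameMode's stock, closing or opening the linked node and its neighbour.
; Placement and removal are blocked while rabbits occupy the slot, with sphere material and decal "Free" parameter showing availability.
; Obstacles take over the slot, deactivating both nodes and refunding any placed fence.
; Destruction reopens the link, decrements total barriers and resets the refill timer to its cooldown.
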(event EventBeginPlay
  (Variables|Default|SetGameMode (.AsBP%20Game%20Mode (Utilities|Casting|CastToBP_GameMode (Game|GetGameMode))))
  (Rendering|SetVisibility (Variables|Default|GetFence) false false)
  (Input|EnableInput (Game|GetPlayerController 0))
  (bind _returnvalue (Rendering|Material|CreateDynamicMaterialInstance (Variables|Default|GetDecal) :!class /Script/Engine.DecalComponent))
  (Variables|Default|SetMID_DecalOutline _returnvalue))

(fn ConstructionScript)

(fn Place/Remove
  (bind _gamemode (Variables|Default|GetGameMode))
  (bind _gamemode_2 (Variables|Default|GetGameMode))
  (bind _linkednode (Variables|Default|GetLinkedNode))
  (bind _linkednode_2 (Variables|Default|GetLinkedNode))
  (if (Variables|Default|GetActivable)
    (if (not (Variables|Default|GetActive))
      (bind _canplace (Default|PlaceBarrier _gamemode true))
      (if _canplace
        (bind _output_get (Variables|Default|SetActive true))
        (Rendering|SetVisibility (Variables|Default|GetFence) _output_get false)
        (Rendering|SetVisibility (Variables|Default|GetSphere) (not (Variables|Default|GetActive)) false)
        (Variables|/Game/PlaceHolder/BP_PathNode.BP_PathNode_C|SetIsOpen _linkednode_2 (not (Variables|Default|GetActive)))
        (Variables|/Game/PlaceHolder/BP_PathNode.BP_PathNode_C|SetIsOpen (Variables|/Game/PlaceHolder/BP_PathNode.BP_PathNode_C|GetNeighbour _linkednode_2) (not (Variables|Default|GetActive)))
        (Rendering|Material|SetScalarParameterValue (Variables|Default|GetMID_DecalOutline) "Free" (Math|Conversions|ToFloat(Boolean) (not (Variables|Default|GetActive))) :!class /Script/Engine.MaterialInstanceDynamic :!label _label)
        (Default|SetMPCCanPlaceFence _gamemode_2 (> (Variables|/Game/Blueprints/BP_GameMode.BP_GameMode_C|GetStockBarrier _gamemode_2) 0)))
      (else
        (bind _canplace_2 (Default|PlaceBarrier _gamemode false))
        (if _canplace_2
          (bind _output_get_2 (Variables|Default|SetActive false))
          (Rendering|SetVisibility (Variables|Default|GetFence) _output_get_2 false)
          (Rendering|SetVisibility (Variables|Default|GetSphere) (not (Variables|Default|GetActive)) false)
          (Variables|/Game/PlaceHolder/BP_PathNode.BP_PathNode_C|SetIsOpen _linkednode (not (Variables|Default|GetActive)))
          (Variables|/Game/PlaceHolder/BP_PathNode.BP_PathNode_C|SetIsOpen (Variables|/Game/PlaceHolder/BP_PathNode.BP_PathNode_C|GetNeighbour _linkednode) (not (Variables|Default|GetActive)))
          (goto _label))))))

(fn ChangeRabbit
  (params (Entering :type Boolean))
  (bind _rabbitin (Variables|Default|GetRabbitIn))
  (if Entering
    (Math|Integer|IncrementInt _rabbitin
      (:%20%20
        _))
    (else
      (Math|Integer|DecrementInt _rabbitin
        (:%20%20
          _))))
  (bind _output_get (Variables|Default|SetActivable (== _rabbitin 0)))
  (Rendering|Material|SetMaterial (Variables|Default|GetSphere) 0 (select _output_get "/Game/PlaceHolder/M_Green.M_Green" "/Game/PlaceHolder/M_Red.M_Red"))
  (Rendering|Material|SetScalarParameterValue (Variables|Default|GetMID_DecalOutline) "Free" (Math|Conversions|ToFloat(Boolean) (Variables|Default|GetActivable)) :!class /Script/Engine.MaterialInstanceDynamic))

(fn ChangeObstacle
  (params (ActivateObstacle :type Boolean))
  (bind _gamemode (Variables|Default|GetGameMode))
  (bind _linkednode (Variables|Default|GetLinkedNode))
  (bind _linkednode_2 (Variables|Default|GetLinkedNode))
  (Rendering|SetVisibility (Variables|Default|GetObstacle) ActivateObstacle false)
  (if (and (Variables|Default|GetActive) (not (Variables|Default|GetObstacleActive)))
    (|RecoverBarrier))
  (if ActivateObstacle
    (Variables|Default|SetObstacleActive ActivateObstacle)
    (Variables|Default|SetActive ActivateObstacle)
    (Variables|/Game/PlaceHolder/BP_PathNode.BP_PathNode_C|SetIsActive _linkednode_2 false)
    (Variables|/Game/PlaceHolder/BP_PathNode.BP_PathNode_C|SetIsActive (Variables|/Game/PlaceHolder/BP_PathNode.BP_PathNode_C|GetNeighbour _linkednode_2) false)
    (Development|PrintString "active obstacle" true true "(R=0.000000,G=1.000000,B=0.148475,A=1.000000)" 1e+01)
    (else
      (Variables|Default|SetObstacleActive ActivateObstacle)
      (Variables|Default|SetActive ActivateObstacle)
      (Variables|/Game/PlaceHolder/BP_PathNode.BP_PathNode_C|SetIsActive _linkednode true)
      (Variables|/Game/PlaceHolder/BP_PathNode.BP_PathNode_C|SetIsActive (Variables|/Game/PlaceHolder/BP_PathNode.BP_PathNode_C|GetNeighbour _linkednode) true)
      (Development|PrintString "deactive obstacle" true true "(R=1.000000,G=0.019096,B=0.000000,A=1.000000)" 1e+01)))
  (Rendering|Material|SetScalarParameterValue (Variables|Default|GetMID_DecalOutline) "Free" (Math|Conversions|ToFloat(Boolean) (not (Variables|Default|GetActive))) :!class /Script/Engine.MaterialInstanceDynamic)
  (Default|SetMPCCanPlaceFence _gamemode (> (Variables|/Game/Blueprints/BP_GameMode.BP_GameMode_C|GetStockBarrier _gamemode) 0)))

(fn Destruct
  (bind _linkednode (Variables|Default|GetLinkedNode))
  (bind _gamemode (Variables|Default|GetGameMode))
  (bind _output_get (Variables|Default|SetActive false))
  (Rendering|SetVisibility (Variables|Default|GetFence) _output_get false)
  (Rendering|SetVisibility (Variables|Default|GetSphere) (not (Variables|Default|GetActive)) false)
  (Variables|/Game/PlaceHolder/BP_PathNode.BP_PathNode_C|SetIsOpen _linkednode (not (Variables|Default|GetActive)))
  (Variables|/Game/PlaceHolder/BP_PathNode.BP_PathNode_C|SetIsOpen (Variables|/Game/PlaceHolder/BP_PathNode.BP_PathNode_C|GetNeighbour _linkednode) (not (Variables|Default|GetActive)))
  (Variables|/Game/Blueprints/BP_GameMode.BP_GameMode_C|SetRefillTimer _gamemode (Variables|/Game/Blueprints/BP_GameMode.BP_GameMode_C|GetRefillCooldown _gamemode))
  (Math|Integer|DecrementInt (Variables|/Game/Blueprints/BP_GameMode.BP_GameMode_C|GetTotalBarrier _gamemode)))